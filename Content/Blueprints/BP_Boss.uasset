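; Two-phase boss enemy that shoots BP_BossBullet projectiles relative to the player's position.
; A looping timer calls BossLoopFunc, which switches on BossState to fire one yaw-offset bullet in Phase 1 or an asymmetric three-bullet spread in Phase 2.
; Each bullet's Direction comes from rotating the boss-to-player vector.
; TakeDamage reduces HP, enters Phase 2 at half health, and at zero destroys the boss with explosion VFX and sound.
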(event `self.ReceiveBeginPlay`
  ; 보스 페이드 및 총알 발사 루프
  (set `self.Boss_HP` (`self.Boss_MaxHP`))
  (set `self.Boss_IsDead` false)
  (set `self.Boss_State` "NewEnumerator0")
  (`KismetSystemLibrary.K2_SetTimer` null "BossLoopFunc" (`KismetMathLibrary.Conv_IntToDouble` (`self.FireInterval`)) true))

(fn `BossLoopFunc`
  ; 보스 1,2 페이즈 넘어가기
  (switch `/Game/Blueprints/E_BossState` (`self.Boss_State`)
    (:`NewEnumerator0`
      (`self.FireStraight`))
    (:`NewEnumerator1`
      (`self.FireSpread`))))

(fn `FireSpread`
  (bind _returnvalue (`self.K2_GetActorLocation`))
  (bind _returnvalue_2 (`GameplayStatics.GetPlayerPawn` 0))
  (bind _returnvalue_3 (`KismetMathLibrary.MakeRotFromX` (`KismetMathLibrary.Normal` (- (`self.K2_GetActorLocation` _returnvalue_2) _returnvalue))))
  (bind _returnvalue_4 (`KismetMathLibrary.MakeTransform` (+ (* (`KismetMathLibrary.GetForwardVector` _returnvalue_3) (`KismetMathLibrary.Conv_DoubleToVector` 50.0)) _returnvalue)))
  ; 보스2페이즈 총알 패턴(분산형)
  (`/Engine/EditorBlueprintResources/StandardMacros.IsValid` _returnvalue_2
    (:`Is Valid`
      (`|ExecutionSequence`
        (:`then_0`
          (bind _returnvalue_5 (`|SpawnActorFromClass` "/Game/Blueprints/BP_BossBullet.BP_BossBullet_C" _returnvalue_4 "Undefined" "MultiplyWithRoot" null null))
          (set `/Game/Blueprints/BP_BossBullet.Direction` (`KismetMathLibrary.GetForwardVector` (`KismetMathLibrary.ComposeRotators` _returnvalue_3 (`KismetMathLibrary.MakeRotator` 0.0 0.0 -20.0))) _returnvalue_5))
        (:`then_1`
          (bind _returnvalue_6 (`|SpawnActorFromClass` "/Game/Blueprints/BP_BossBullet.BP_BossBullet_C" _returnvalue_4 "Undefined" "MultiplyWithRoot" null null))
          (set `/Game/Blueprints/BP_BossBullet.Direction` (`KismetMathLibrary.GetForwardVector` (`KismetMathLibrary.ComposeRotators` _returnvalue_3 (`KismetMathLibrary.MakeRotator` 0.0 0.0 50.0))) _returnvalue_6))
        (:`then_2`
          (bind _returnvalue_7 (`|SpawnActorFromClass` "/Game/Blueprints/BP_BossBullet.BP_BossBullet_C" _returnvalue_4 "Undefined" "MultiplyWithRoot" null null))
          (set `/Game/Blueprints/BP_BossBullet.Direction` (`KismetMathLibrary.GetForwardVector` (`KismetMathLibrary.ComposeRotators` _returnvalue_3 (`KismetMathLibrary.MakeRotator` 0.0 0.0 100.0))) _returnvalue_7))))))

(fn `FireStraight`
  (bind _returnvalue (`self.K2_GetActorLocation`))
  (bind _returnvalue_2 (`GameplayStatics.GetPlayerPawn` 0))
  (bind _returnvalue_3 (`KismetMathLibrary.GetForwardVector` (`KismetMathLibrary.ComposeRotators` (`KismetMathLibrary.MakeRotFromX` (`KismetMathLibrary.Normal` (- (`self.K2_GetActorLocation` _returnvalue_2) _returnvalue))) (`KismetMathLibrary.MakeRotator` 0.0 0.0 20.0))))
  ; 보스 총알 생성
  (`/Engine/EditorBlueprintResources/StandardMacros.IsValid` _returnvalue_2
    (:`Is Valid`
      (bind _returnvalue_4 (`|SpawnActorFromClass` "/Game/Blueprints/BP_BossBullet.BP_BossBullet_C" (`KismetMathLibrary.MakeTransform` (+ (* _returnvalue_3 (`KismetMathLibrary.Conv_DoubleToVector` 50.0)) _returnvalue)) "Undefined" "MultiplyWithRoot" null null))
      (set `/Game/Blueprints/BP_BossBullet.Direction` _returnvalue_3 _returnvalue_4))))

(fn `TakeDamage`
  (params (Damage :type "Float (double-precision)"))
  ; 보스가 대미지를 받음
  (bind _output_get (set `self.BossHP` (- (`self.BossHP`) Damage)))
  (if (<= _output_get 0.0)
    (`self.K2_DestroyActor`)
    (`NiagaraFunctionLibrary.SpawnSystemAtLocation` "/Game/Fire_EXP_Vol01_Free/Niagara/EXP/NS_Sub_EXP_Large_001_01.NS_Sub_EXP_Large_001_01" (`self.K2_GetActorLocation`))
    (`GameplayStatics.PlaySound2D` "/Game/Explosion.Explosion" 1.0 1.0 0.0 null null)
    (else
      ;; 보스 피가 절반일 시 페이즈2로 넘어감
      (if (<= (`self.BossHP`) (* 0.5 (`self.Boss_MaxHP`)))
        (set `self.Boss_State` "NewEnumerator1")
        (`KismetSystemLibrary.PrintString` "페이즈2 넘어감")))))

(fn `UserConstructionScript`)