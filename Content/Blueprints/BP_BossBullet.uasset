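; BP_BossBullet is a projectile actor, named as a boss's bullet, that kills the player on contact.
; Each Tick it moves along its normalized Direction scaled by Speed and delta time, using a swept SetActorLocation rather than a movement component.
; When its Cube component begins overlapping a BP_Player, it calls PlayerDie on that player.
; A short lifespan set on BeginPlay removes the bullet, which is not destroyed on hit.
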(event `self.ReceiveBeginPlay`
  (`self.SetLifeSpan` 3.0))

(event `self.ReceiveTick`
  (params (DeltaSeconds :type "Float (single-precision)"))
  ; 이동한다.
  (`self.K2_SetActorLocation` (+ (* DeltaSeconds (* (`KismetMathLibrary.Normal` (`self.Direction`)) (`self.Speed`))) (`self.K2_GetActorLocation`)) true))

(event `self.Cube.OnComponentBeginOverlap`
  (params (OverlappedComponent :type "PrimitiveComponent Object Reference") (OtherActor :type "Actor Object Reference") (OtherComp :type "PrimitiveComponent Object Reference") (OtherBodyIndex :type Integer) (bFromSweep :type Boolean) (SweepResult :type "HitResult Structure (by ref)"))
  (bind _asbp_player (cast `/Game/Blueprints/BP_Player` OtherActor))
  (`/Game/Blueprints/BP_Player.Player_Die` _asbp_player))

(fn `UserConstructionScript`)