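; BP_Bullet is a projectile actor that damages the boss on contact.
; Every tick it moves along its Direction at Speed, using a non-sweeping location update scaled by delta time.
; When its Cube overlaps a BP_Boss it passes Damage to the boss's TakeDamage and destroys itself.
; Overlapping a BP_Enemy only destroys the bullet, and its own TakeDamage function is empty.
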(event `self.ReceiveBeginPlay`)

(event `self.ReceiveTick`
  (params (DeltaSeconds :type "Float (single-precision)"))
  ; 이동한다.
  (`self.K2_SetActorLocation` (+ (* DeltaSeconds (* (`self.Direction`) (`self.Speed`))) (`self.K2_GetActorLocation`))))

(event `self.Cube.OnComponentBeginOverlap`
  (params (OverlappedComponent :type "PrimitiveComponent Object Reference") (OtherActor :type "Actor Object Reference") (OtherComp :type "PrimitiveComponent Object Reference") (OtherBodyIndex :type Integer) (bFromSweep :type Boolean) (SweepResult :type "HitResult Structure (by ref)"))
  ; 보스 데미지 주기
  (bind _asbp_boss (cast `/Game/Blueprints/BP_Boss` OtherActor)
    (:`then`
      (`/Game/Blueprints/BP_Boss.TakeDamage` _asbp_boss (`self.Damage`))
      (`self.K2_DestroyActor`))
    (:`CastFailed`
      (cast `/Game/Blueprints/BP_Enemy` OtherActor)
      (`self.K2_DestroyActor`))))

(fn `TakeDamage`)

(fn `UserConstructionScript`)