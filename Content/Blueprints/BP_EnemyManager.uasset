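; Enemy spawner that periodically creates BP_Enemy at its own location and triggers the boss fight.
; Tick accumulates time past CreateTime, spawns while the game instance allows it, and gives each enemy a back-reference to the manager.
; EnemyKilled increments the global kill count; at ten, if CanSpawnBoss is set, it halts enemy spawning and spawns BP_Boss once at the first BP_BossPoint found on BeginPlay.
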(event `self.ReceiveBeginPlay`
  (bind _outactors (`GameplayStatics.GetAllActorsOfClass` "/Game/Blueprints/BP_BossPoint.BP_BossPoint_C"))
  (set `self.BossSpawnRef` (`|GetArrayItem` _outactors)))

(event `self.ReceiveTick`
  (params (DeltaSeconds :type "Float (single-precision)"))
  ; 시간이 흐른다.
  (bind _output_get (set `self.CurrentTime` (+ DeltaSeconds (`self.CurrentTime`))))
  ; 생성시간이 됐으니까
  (if (> _output_get (`self.CreateTime`))
    (bind _asbp_my_game_istance (cast `/Game/Blueprints/BP_MyGameIstance` (`GameplayStatics.GetGameInstance`)))
    ; 적생성
    (if (`/Game/Blueprints/BP_MyGameIstance.GlobalCanSpawnEnemies` _asbp_my_game_istance)
      (bind _returnvalue (`|SpawnActorFromClass` "/Game/Blueprints/BP_Enemy.BP_Enemy_C" (`KismetMathLibrary.MakeTransform` (`self.K2_GetActorLocation`)) "AlwaysSpawn" "MultiplyWithRoot" null null))
      (`/Engine/EditorBlueprintResources/StandardMacros.IsValid` _returnvalue
        (:`Is Valid`
          (set `/Game/Blueprints/BP_Enemy.EnemyManagerRef` self _returnvalue)
          (set `self.CurrentTime` 0.0))))))

(fn `EnemyKilled`
  ; 적 10명 죽을 시 보스 생성
  (bind _asbp_my_game_istance (cast `/Game/Blueprints/BP_MyGameIstance` (`GameplayStatics.GetGameInstance`)))
  (bind _output_get (set `/Game/Blueprints/BP_MyGameIstance.GlobalKillCount` (+ (`/Game/Blueprints/BP_MyGameIstance.GlobalKillCount` _asbp_my_game_istance) 1) _asbp_my_game_istance))
  (if (and (>= _output_get 10) (not (`/Game/Blueprints/BP_MyGameIstance.GlobalBossSpawned` _asbp_my_game_istance)) (`self.CanSpawnBoss`))
    (set `/Game/Blueprints/BP_MyGameIstance.GlobalBossSpawned` true _asbp_my_game_istance)
    (set `/Game/Blueprints/BP_MyGameIstance.GlobalCanSpawnEnemies` false _asbp_my_game_istance)
    (`|SpawnActorFromClass` "/Game/Blueprints/BP_Boss.BP_Boss_C" (`KismetMathLibrary.MakeTransform` (`self.K2_GetActorLocation` (`self.BossSpawnRef`))) "Undefined" "MultiplyWithRoot" null null)))

(fn `UserConstructionScript`)